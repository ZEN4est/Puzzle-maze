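; BP_IconShowed is an actor that shows an interaction icon widget while the first-person character is inside its trigger area.
; On BeginPlay it offsets the widget component and passes its brush and text to the W_EInteract widget.
; Begin and end overlaps on IconShowedCollider set InRange, which drives the widget's visibility, and print debug strings.
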(event `self.ReceiveBeginPlay`
  (bind _widget (`self.Widget`))
  ;[1 1 1] SetIcon
  (`SceneComponent.K2_AddWorldOffset` _widget (`self.IconLocationTransform`) false false)
  (bind _asw_einteract (cast `/Game/Main/UI/InteractButtons/W_EInteract` (`WidgetComponent.GetWidget` _widget)))
  (set `/Game/Main/UI/InteractButtons/W_EInteract.Brush` (`self.IconBrush`) _asw_einteract)
  (set `/Game/Main/UI/InteractButtons/W_EInteract.IconText` (`self.IconText`) _asw_einteract))

(event `self.IconShowedCollider.OnComponentBeginOverlap`
  (params (OverlappedComponent :type "PrimitiveComponent Object Reference") (OtherActor :type "Actor Object Reference") (OtherComp :type "PrimitiveComponent Object Reference") (OtherBodyIndex :type Integer) (bFromSweep :type Boolean) (SweepResult :type "HitResult Structure (by ref)"))
  (cast `/Game/FirstPerson/Blueprints/BP_FirstPersonCharacter` OtherActor)
  (bind _output_get (set `self.InRange` true))
  (`SceneComponent.SetVisibility` (`self.Widget`) _output_get false)
  (`KismetSystemLibrary.PrintString` "In"))

(event `self.IconShowedCollider.OnComponentEndOverlap`
  (params (OverlappedComponent :type "PrimitiveComponent Object Reference") (OtherActor :type "Actor Object Reference") (OtherComp :type "PrimitiveComponent Object Reference") (OtherBodyIndex :type Integer))
  (cast `/Game/FirstPerson/Blueprints/BP_FirstPersonCharacter` OtherActor)
  (bind _output_get (set `self.InRange` false))
  (`SceneComponent.SetVisibility` (`self.Widget`) _output_get false)
  (`KismetSystemLibrary.PrintString` "Out"))

(fn `UserConstructionScript`)