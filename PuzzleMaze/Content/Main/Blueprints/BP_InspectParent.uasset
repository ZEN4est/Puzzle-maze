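; Base actor for inspectable items that the player picks up and views in front of the camera.
; On interact, if nothing is held, it hands input from the player to itself, attaches to the player's Item component, disables physics and moves to DistanceToCamera along the camera's forward vector.
; IA_StopInspect returns input, resets the relative transform, detaches with physics restored and clears CurrentItemHeld.
; IsLookingAt is a stub returning false.
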(event `/Game/Main/Blueprints/Interfaces/BPI_Inspect.InteractWith`
  (params (PlayerControler :type "/Game/FirstPerson/Blueprints/BP_FirstPersonCharacter Object Reference"))
  (`KismetSystemLibrary.PrintString` "EventInteractWith")
  (bind _output_get (set `self.Player Controler` PlayerControler))
  (`/Game/FirstPerson/Blueprints/BP_FirstPersonCharacter.CurrentItemHeld` _output_get
    (:`then`)
    (:`else`
      (`self.StartInspection`))))

(event `EnhancedInput|/Game/FirstPerson/Input/Actions/IA_StopInspect`
  (params (ActionValue :type Boolean) (ElapsedSeconds :type "Float (double-precision)") (TriggeredSeconds :type "Float (double-precision)") (InputAction :type "InputAction Object Reference" :default "/Game/FirstPerson/Input/Actions/IA_StopInspect.IA_StopInspect"))
  (:`Triggered`
    (`KismetSystemLibrary.PrintString` "EventStopInspect")
    (`self.StopInspection`)
    (set `/Game/FirstPerson/Blueprints/BP_FirstPersonCharacter.CurrentItemHeld` null (stale `/Game/Main/Blueprints/Interfaces/BPI_Inspect.InteractWith` _output_get))))

(fn `IsLookingAt?`
  (returns (`IsLookingAt?` :type Boolean))
  (return false))

(fn `StartInspection`
  (bind _returnvalue (`GameplayStatics.GetPlayerCameraManager` 0))
  (bind _returnvalue_2 (`GameplayStatics.GetPlayerController` 0))
  (bind _collider (`self.Collider`))
  (bind _player_controler (`self.Player Controler`))
  (`KismetSystemLibrary.PrintString` "StartInspection")
  (`self.DisableInput` _player_controler _returnvalue_2)
  (`self.EnableInput` _returnvalue_2)
  (`self.K2_AttachToComponent` (`/Game/FirstPerson/Blueprints/BP_FirstPersonCharacter.Item` _player_controler) "None" "SnapToTarget" "SnapToTarget" "KeepRelative")
  (`PrimitiveComponent.SetSimulatePhysics` _collider false)
  (`PrimitiveComponent.SetCollisionEnabled` _collider "QueryAndPhysics")
  (set `/Game/FirstPerson/Blueprints/BP_FirstPersonCharacter.CurrentItemHeld` self (`self.Player Controler`))
  (`self.K2_SetActorLocation` (+ (`PlayerCameraManager.GetCameraLocation` _returnvalue) (* (`KismetMathLibrary.GetForwardVector` (`PlayerCameraManager.GetCameraRotation` _returnvalue)) (`self.DistanceToCamera`))))
  (`KismetSystemLibrary.PrintString` "inspection started"))

(fn `StopInspection`
  (bind _returnvalue (`GameplayStatics.GetPlayerController` 0))
  (bind _collider (`self.Collider`))
  (`self.DisableInput` _returnvalue)
  (`self.EnableInput` (`self.Player Controler`) _returnvalue)
  (`self.K2_SetActorRelativeLocation` (0.0 0.0 0.0))
  (`self.K2_SetActorRelativeRotation` (struct))
  (`self.K2_DetachFromActor` "KeepWorld" "KeepWorld" "KeepWorld")
  (`PrimitiveComponent.SetCollisionEnabled` _collider "QueryAndPhysics")
  (`PrimitiveComponent.SetSimulatePhysics` _collider true))

(fn `UserConstructionScript`)