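; Three-digit combination lock that the player operates in a close-up view.
; Interacting while BP_IconShowed reports LookingAt blends the view to the lock and disables first-person controller input; QuitCombo reverses this.
; Left/Right select a wheel, Tick highlights it by material swap, and Interact rotates it one step, rebuilding the entered number.
; Approve compares that number to Code, and a match clears IsLocked, exits the view and removes the icon components.
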(event `self.ReceiveBeginPlay`
  (bind _returnvalue (`GameplayStatics.GetPlayerController` 0))
  (`self.EnableInput` _returnvalue)
  (set `self.PlayerController` _returnvalue))

(event `Key|Right`
  (params (Key :type "Key Structure"))
  ;[1 1 1] IncreaseSelection
  (:`Pressed`
    (if (`self.AbleToWork`)
      (bind _output_get (set `self.Selected_Id` (mod (`KismetMathLibrary.Abs_Int` (+ (`self.Selected_Id`) 1)) 3)))
      (`KismetSystemLibrary.PrintString` (`KismetStringLibrary.Concat_StrStr` "Zwiekszono wartosc, nowa to: " (`KismetStringLibrary.Conv_IntToString` _output_get))))))

(event `Key|Left`
  (params (Key :type "Key Structure"))
  ;[1 1 1] DecreaseSelection
  (:`Pressed`
    (if (`self.AbleToWork`)
      (bind _output_get (set `self.Selected_Id` (mod (`KismetMathLibrary.Abs_Int` (+ (`self.Selected_Id`) 2)) 3)))
      (`KismetSystemLibrary.PrintString` (`KismetStringLibrary.Concat_StrStr` "Zmniejszono wartosc, nowa to: " (`KismetStringLibrary.Conv_IntToString` _output_get))))))

(event `EnhancedInput|/Game/FirstPerson/Input/Actions/IA_Interact`
  (params (ActionValue :type Boolean) (ElapsedSeconds :type "Float (double-precision)") (TriggeredSeconds :type "Float (double-precision)") (InputAction :type "InputAction Object Reference" :default "/Game/FirstPerson/Input/Actions/IA_Interact.IA_Interact"))
  ;[1 1 1] SettingDigits
  ;;[1 1 1] Changing digits
  (:`Started`
    (if (`self.IsLocked`)
      (if (`self.AbleToWork`)
        (`/Engine/EditorBlueprintResources/StandardMacros.Gate` true :!label _label
          (:`Exit`
            (`self.SetDigit` (`self.Selected_Id`))))))))

(event `self.ReceiveTick`
  (params (DeltaSeconds :type "Float (single-precision)"))
  ;[1 1 1] SettingDigits
  (if (`self.IsLocked`)
    (if (`self.AbleToWork`)
      ;;[1 1 1] SwitchingSelection
      (switch `int` (`self.Selected_Id`)
        (:`0`
          (`self.ResetSelection`)
          (`PrimitiveComponent.SetMaterial` (`self.Digit_0`) 0 "/Game/Main/Assets/Objects/ComboLock/Digits_Selected.Digits_Selected")
          (goto _label :!via `Open`))
        (:`1`
          (`self.ResetSelection`)
          (`PrimitiveComponent.SetMaterial` (`self.Digit_1`) 0 "/Game/Main/Assets/Objects/ComboLock/Digits_Selected.Digits_Selected")
          (goto _label :!via `Open`))
        (:`2`
          (`self.ResetSelection`)
          (`PrimitiveComponent.SetMaterial` (`self.Digit_2`) 0 "/Game/Main/Assets/Objects/ComboLock/Digits_Selected.Digits_Selected")
          (goto _label :!via `Open`))))))

(event `EnhancedInput|/Game/FirstPerson/Input/Actions/IA_Interact`
  (params (ActionValue :type Boolean) (ElapsedSeconds :type "Float (double-precision)") (TriggeredSeconds :type "Float (double-precision)") (InputAction :type "InputAction Object Reference" :default "/Game/FirstPerson/Input/Actions/IA_Interact.IA_Interact"))
  (bind _playercontroller (`self.PlayerController`))
  ;[1 1 1] EnterCombo
  (:`Started`
    (if (`self.IsLocked`)
      (if (`/Game/Main/Blueprints/BP_IconShowed.LookingAt?` (`self.IconShowedInstance`))
        (set `self.AbleToWork` true)
        (`PlayerController.SetViewTargetWithBlend` (`GameplayStatics.GetPlayerController` 0) self 0.0 "VTBlend_Linear" 0.0 false)
        (`SceneComponent.SetVisibility` (`self.ComboIconSet`) true false)
        (`Widget.SetVisibility` (`WidgetComponent.GetWidget` (`/Game/Main/Blueprints/BP_IconShowed.Widget` (`self.IconShowedInstance`))) "Hidden")
        (`self.EnableInput` _playercontroller)
        (bind _asbp_first_person_player_controller (cast `/Game/FirstPerson/Blueprints/BP_FirstPersonPlayerController` _playercontroller))
        (`self.DisableInput` _asbp_first_person_player_controller _playercontroller)))))

(event `EnhancedInput|/Game/FirstPerson/Input/Actions/IA_QButton`
  (params (ActionValue :type Boolean) (ElapsedSeconds :type "Float (double-precision)") (TriggeredSeconds :type "Float (double-precision)") (InputAction :type "InputAction Object Reference" :default "/Game/FirstPerson/Input/Actions/IA_QButton.IA_QButton"))
  ;[1 1 1] QuitCombo
  (:`Triggered`
    (if (`self.IsLocked`)
      (`self.QuitCombo`))))

(event `EnhancedInput|/Game/FirstPerson/Input/Actions/IA_Approve`
  (params (ActionValue :type Boolean) (ElapsedSeconds :type "Float (double-precision)") (TriggeredSeconds :type "Float (double-precision)") (InputAction :type "InputAction Object Reference" :default "/Game/FirstPerson/Input/Actions/IA_Approve.IA_Approve"))
  ;[1 1 1] Approve Digits
  (:`Started`
    (if (`self.IsLocked`)
      (if (== (`self.Digit_set`) (`self.Code`))
        (set `self.IsLocked` false)
        (`self.QuitCombo`)
        (`ActorComponent.K2_DestroyComponent` (`self.ComboIconSet`))
        (`ActorComponent.K2_DestroyComponent` (`self.BP_IconShowed`))))))

(fn `QuitCombo`
  (bind _playercontroller (`self.PlayerController`))
  (if (`/Game/Main/Blueprints/BP_IconShowed.LookingAt?` (`self.IconShowedInstance`))
    (set `self.AbleToWork` false)
    (`self.ResetSelection`)
    (`PlayerController.SetViewTargetWithBlend` (`GameplayStatics.GetPlayerController` 0) (`GameplayStatics.GetPlayerCharacter` 0) 0.0 "VTBlend_Linear" 0.0 false)
    (`SceneComponent.SetVisibility` (`self.ComboIconSet`) false false)
    (`Widget.SetVisibility` (`WidgetComponent.GetWidget` (`/Game/Main/Blueprints/BP_IconShowed.Widget` (`self.IconShowedInstance`))) "Visible")
    (bind _asbp_first_person_player_controller (cast `/Game/FirstPerson/Blueprints/BP_FirstPersonPlayerController` _playercontroller))
    (`self.EnableInput` _asbp_first_person_player_controller _playercontroller)))

(fn `ResetSelection`
  (`PrimitiveComponent.SetMaterial` (`self.Digit_0`) 0 "/Game/Main/Assets/Objects/ComboLock/Digits.Digits")
  (`PrimitiveComponent.SetMaterial` (`self.Digit_1`) 0 "/Game/Main/Assets/Objects/ComboLock/Digits.Digits")
  (`PrimitiveComponent.SetMaterial` (`self.Digit_2`) 0 "/Game/Main/Assets/Objects/ComboLock/Digits.Digits"))

(fn `SetDigit`
  (params (ObjectID :type Integer))
  (switch `int` ObjectID
    (:`0`
      (`SceneComponent.K2_AddLocalRotation` (`self.Digit_0`) (struct :`Pitch` -36.0) false false)
      (bind _output_get (set `self.Digit_0_set` (mod (+ (`self.Digit_0_set`) 1) 10))))
    (:`1`
      (`SceneComponent.K2_AddLocalRotation` (`self.Digit_1`) (struct :`Pitch` -36.0) false false)
      (bind _output_get_2 (set `self.Digit_1_set` (mod (+ (`self.Digit_1_set`) 1) 10))))
    (:`2`
      (`SceneComponent.K2_AddLocalRotation` (`self.Digit_2`) (struct :`Pitch` -36.0) false false)
      (bind _output_get_3 (set `self.Digit_2_set` (mod (+ (`self.Digit_2_set`) 1) 10)))))
  (bind _output_get_4 (set `self.Digit_set` (+ (* _output_get 100) (* _output_get_2 10) _output_get_3)))
  (`KismetSystemLibrary.PrintString` (`KismetStringLibrary.Concat_StrStr` "Wyprana liczba: " (`KismetStringLibrary.Conv_IntToString` _output_get_4))))

(fn `UserConstructionScript`
  (bind _asbp_icon_showed (cast `/Game/Main/Blueprints/BP_IconShowed` (`ChildActorComponent.ChildActor` (`self.BP_IconShowed`))))
  (set `self.IconShowedInstance` _asbp_icon_showed))