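; BP_Box is a box that reveals a key item when opened.
; On BeginPlay it enables query and physics collision on its Box1 mesh.
; The OpenBox event plays a one-shot open animation, waits briefly, then spawns a BP_Equipable at an offset from the box, with hard-coded chest key item data passed in at spawn.
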(event `self.ReceiveBeginPlay`
  (`PrimitiveComponent.SetCollisionEnabled` (`self.Box1`) "QueryAndPhysics"))

(event `OpenBox`
  (`SkeletalMeshComponent.PlayAnimation` (`self.Box1`) "/Game/Main/Assets/Box1_Anim.Box1_Anim" false)
  (`KismetSystemLibrary.Delay` 0.5)
  (`|SpawnActorFromClass` "/Game/Main/Blueprints/InventorySystem/BP_Equipable.BP_Equipable_C" (`KismetMathLibrary.Conv_VectorToTransform` (+ (`SceneComponent.K2_GetComponentLocation` (`self.Box1`)) (0.0 40.0 -15.0))) "Undefined" "MultiplyWithRoot" null (make `/Game/Main/Blueprints/InventorySystem/S_InInventoryItem` "Key" "Key to chest" (make `SlateBrush` "Image" "NoTile" "NoMirror" (struct :`X` 32.0 :`Y` 32.0) (struct) (struct :`SpecifiedColor` (struct :`R` 1.0 :`G` 1.0 :`B` 1.0 :`A` 1.0) :`ColorUseRule` "UseColor_Specified") (struct :`CornerRadii` (struct) :`Color` (struct :`SpecifiedColor` (struct) :`ColorUseRule` "UseColor_Specified") :`RoundingType` "HalfHeightRadius") "/Game/Main/Images/Key_Icon.Key_Icon") (1.0 1.0 1.0) (struct) "/Game/Main/Assets/Objects/Key.Key" (0.0 0.0 0.0) (struct) (1.0 1.0 1.0) 15 0 false null) null))

(fn `UserConstructionScript`)