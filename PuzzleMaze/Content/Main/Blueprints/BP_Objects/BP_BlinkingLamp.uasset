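; Lamp actor that flickers its light in a fixed, scripted blinking pattern.
; BeginPlay runs a long hard-coded chain of Delays that switch the Rx light's intensity between off and full brightness, with irregular short and long intervals.
; The chain loops back to its start indefinitely, with a longer dark pause opening each cycle.
; The construction script only calls its parent.
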(event `self.ReceiveBeginPlay`
  (bind _rx (`self.rx`))
  (bind _rx_2 (`self.rx`))
  (bind _rx_3 (`self.rx`))
  (`LightComponent.SetIntensity` _rx 0.0 :!label _label)
  (`KismetSystemLibrary.Delay` 5.0)
  (`LightComponent.SetIntensity` _rx 0.0)
  (`KismetSystemLibrary.Delay` 0.1)
  (`LightComponent.SetIntensity` _rx 5000.0)
  (`KismetSystemLibrary.Delay` 0.5)
  (`LightComponent.SetIntensity` _rx 0.0)
  (`KismetSystemLibrary.Delay` 0.1)
  (`LightComponent.SetIntensity` _rx 5000.0)
  (`KismetSystemLibrary.Delay` 0.5)
  (`LightComponent.SetIntensity` _rx 0.0)
  (`KismetSystemLibrary.Delay` 0.1)
  (`LightComponent.SetIntensity` _rx 5000.0)
  (`KismetSystemLibrary.Delay` 0.5)
  (`LightComponent.SetIntensity` _rx 0.0)
  (`KismetSystemLibrary.Delay` 0.1)
  (`LightComponent.SetIntensity` _rx 5000.0)
  (`KismetSystemLibrary.Delay` 1.5)
  (`LightComponent.SetIntensity` _rx 0.0)
  (`KismetSystemLibrary.Delay` 0.1)
  (`LightComponent.SetIntensity` _rx 5000.0)
  (`KismetSystemLibrary.Delay` 1.5)
  (`LightComponent.SetIntensity` _rx_2 0.0)
  (`KismetSystemLibrary.Delay` 1.5)
  (`LightComponent.SetIntensity` _rx_2 5000.0)
  (`KismetSystemLibrary.Delay` 0.5)
  (`LightComponent.SetIntensity` _rx_2 0.0)
  (`KismetSystemLibrary.Delay` 0.1)
  (`LightComponent.SetIntensity` _rx_2 5000.0)
  (`KismetSystemLibrary.Delay` 0.5)
  (`LightComponent.SetIntensity` _rx_2 0.0)
  (`KismetSystemLibrary.Delay` 0.1)
  (`LightComponent.SetIntensity` _rx_2 5000.0)
  (`KismetSystemLibrary.Delay` 0.5)
  (`LightComponent.SetIntensity` _rx_2 0.0)
  (`KismetSystemLibrary.Delay` 0.1)
  (`LightComponent.SetIntensity` _rx_2 5000.0)
  (`KismetSystemLibrary.Delay` 0.5)
  (`LightComponent.SetIntensity` _rx_2 0.0)
  (`KismetSystemLibrary.Delay` 0.1)
  (`LightComponent.SetIntensity` _rx_2 5000.0)
  (`KismetSystemLibrary.Delay` 0.5)
  (`LightComponent.SetIntensity` _rx_2 0.0)
  (`KismetSystemLibrary.Delay` 0.1)
  (`KismetSystemLibrary.Delay` 1.5)
  (`LightComponent.SetIntensity` _rx_3 5000.0)
  (`KismetSystemLibrary.Delay` 1.5)
  (`LightComponent.SetIntensity` _rx_3 0.0)
  (`KismetSystemLibrary.Delay` 0.1)
  (`LightComponent.SetIntensity` _rx_3 5000.0)
  (`KismetSystemLibrary.Delay` 1.5)
  (`LightComponent.SetIntensity` _rx_3 0.0)
  (`KismetSystemLibrary.Delay` 0.1)
  (`LightComponent.SetIntensity` _rx_3 5000.0)
  (`KismetSystemLibrary.Delay` 1.5)
  (`LightComponent.SetIntensity` _rx_3 0.0)
  (`KismetSystemLibrary.Delay` 0.1)
  (`LightComponent.SetIntensity` _rx_3 5000.0)
  (`KismetSystemLibrary.Delay` 1.5)
  (`LightComponent.SetIntensity` _rx_3 0.0)
  (`KismetSystemLibrary.Delay` 0.1)
  (`LightComponent.SetIntensity` _rx_3 5000.0)
  (`KismetSystemLibrary.Delay` 0.5)
  (`LightComponent.SetIntensity` _rx_3 0.0)
  (`KismetSystemLibrary.Delay` 0.1)
  (goto _label))

(fn `UserConstructionScript`
  (`parent.UserConstructionScript`))