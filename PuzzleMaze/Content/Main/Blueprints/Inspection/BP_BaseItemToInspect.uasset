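; Base actor for world items the player can inspect, with mesh, rotation and scale set from ItemData in the construction script.
; Its widget shows while LookedAt is true, and pressing interact then spawns a far-off BP_InspectedItem, passing it the item's mesh, text, transform settings and equip-button visibility.
; An IsCurrentlyInspecting flag blocks repeat inspections until Q or the game mode's equip-button event clears it.
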(event `self.ReceiveBeginPlay`
  (bind _widget (`self.Widget`))
  (`SceneComponent.K2_SetWorldLocation` _widget (+ (`SceneComponent.K2_GetComponentLocation` _widget) (`.IconTransform_20_1F56282A4BB9D6E1A7FBE0AEEEF52FDF` (break `/Game/Main/Blueprints/InventorySystem/S_InInventoryItem` (`self.ItemData`)))) false false)
  (`self.EnableInput` (`GameplayStatics.GetPlayerController` 0))
  ;[1 1 1] ButtonPressedEvent
  (bind _asbp_first_person_game_mode (cast `/Game/FirstPerson/Blueprints/BP_FirstPersonGameMode` (`GameplayStatics.GetGameMode`)))
  (add `/Game/FirstPerson/Blueprints/BP_FirstPersonGameMode.EquipPressButton` _asbp_first_person_game_mode (delegate `EquipButtonPressed`)))

(event `EquipButtonPressed`
  ;[1 1 1] ButtonPressedEvent
  (set `self.IsCurrentlyInspecting?` false :!label _label))

(event `EnhancedInput|/Game/FirstPerson/Input/Actions/IA_QButton`
  (params (ActionValue :type Boolean) (ElapsedSeconds :type "Float (double-precision)") (TriggeredSeconds :type "Float (double-precision)") (InputAction :type "InputAction Object Reference" :default "/Game/FirstPerson/Input/Actions/IA_QButton.IA_QButton"))
  (:`Started`
    (goto _label)))

(event `EnhancedInput|/Game/FirstPerson/Input/Actions/IA_Interact`
  (params (ActionValue :type Boolean) (ElapsedSeconds :type "Float (double-precision)") (TriggeredSeconds :type "Float (double-precision)") (InputAction :type "InputAction Object Reference" :default "/Game/FirstPerson/Input/Actions/IA_Interact.IA_Interact"))
  (:`Started`
    (if (`self.LookedAt?`)
      (if (not (`self.IsCurrentlyInspecting?`))
        (set `self.IsCurrentlyInspecting?` true)
        (bind _asbp_first_person_character (cast `/Game/FirstPerson/Blueprints/BP_FirstPersonCharacter` (`GameplayStatics.GetPlayerCharacter` 0)))
        (`/Game/Main/Blueprints/Interfaces/BPI_Inspect.Interact` _asbp_first_person_character)))))

(event `self.ReceiveTick`
  (params (DeltaSeconds :type "Float (single-precision)"))
  (`SceneComponent.SetVisibility` (`self.Widget`) (`self.LookedAt?`) false))

(event `/Game/Main/Blueprints/Interfaces/BPI_Inspect.Interact`
  (params (Character :type "/Game/FirstPerson/Blueprints/BP_FirstPersonCharacter Object Reference"))
  (bind (_itemdata_itemname _itemdata_itemdescription _itemdata_itemicon _itemdata_itemscale _itemdata_itemrotation _itemdata_itemmesh _itemdata_icontransform _itemdata_inspectionrotation _itemdata_inspectionscale) (break `/Game/Main/Blueprints/InventorySystem/S_InInventoryItem` (`self.ItemData`)))
  (bind (_itemname _itemdescription _itemicon _itemscale _itemrotation _itemmesh) (break `/Game/Main/Blueprints/InventorySystem/S_InInventoryItem` (`self.ItemData`)))
  (bind _returnvalue (`|SpawnActorFromClass` "/Game/Main/Blueprints/Inspection/BP_InspectedItem.BP_InspectedItem_C" (`KismetMathLibrary.MakeTransform` (100000000.0 0.0 0.0)) "Undefined" "MultiplyWithRoot" null null))
  (`/Game/Main/Blueprints/Inspection/BP_InspectedItem.Set Inspect Rotation` _returnvalue _itemdata_inspectionrotation)
  (`/Game/Main/Blueprints/Inspection/BP_InspectedItem.Set Inspect Scale` _returnvalue _itemdata_inspectionscale)
  (message `/Game/Main/Blueprints/Interfaces/BPI_Inspect.Inspect` _returnvalue Character _itemmesh _itemname _itemdescription (`self.EquipButtonVisibility`)))

(fn `IsLookingAt?`
  (returns (`IsLookingAt?` :type Boolean))
  (return false))

(fn `UserConstructionScript`
  (bind _item (`self.Item`))
  (bind (_itemname _itemdescription _itemicon _itemscale _itemrotation _itemmesh) (break `/Game/Main/Blueprints/InventorySystem/S_InInventoryItem` (`self.ItemData`)))
  (`|ExecutionSequence`
    (:`then_0`
      ;[1 1 1] Setting mesh dynamicaly
      (`StaticMeshComponent.SetStaticMesh` (`self.Item`) _itemmesh)
      ;[1 1 1] Setting scale dynamically
      (`SceneComponent.K2_SetWorldTransform` _item (`KismetMathLibrary.MakeTransform` (`SceneComponent.K2_GetComponentLocation` _item) _itemrotation _itemscale) false false))))