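; BP_Equipable is an inventory item actor that turns into an equipped item when Equip is called.
; Equip removes the item from its weight-based place reference, or from its ID-based one if the first is invalid.
; It then spawns a hard-coded BP_Key far below the world origin, passing on ItemData, and returns it.
; The original actor destroys itself through DestroyItem after a short delay.
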(event `DestroyItem`
  (`KismetSystemLibrary.Delay` 0.1)
  (`self.K2_DestroyActor`))

(fn `Equip`
  (returns (ItemReference :type "/Game/Main/Blueprints/Inspection/BP_BaseItemToInspect Object Reference"))
  (bind _itemdata (`self.ItemData`))
  (bind (_itemdata_itemname _itemdata_itemdescription _itemdata_itemicon _itemdata_itemscale _itemdata_itemrotation _itemdata_itemmesh _itemdata_icontransform _itemdata_inspectionrotation _itemdata_inspectionscale _itemdata_keyid _itemdata_itemid _itemdata_israndomitem_ _itemdata_placereferenceweight _itemdata_placereferenceid) (break `/Game/Main/Blueprints/InventorySystem/S_InInventoryItem` (`self.ItemData`)))
  (`/Engine/EditorBlueprintResources/StandardMacros.IsValid` _itemdata_placereferenceweight
    (:`Is Valid`
      (`/Game/Main/Blueprints/PlaceForItemSystem/BP_PlaceForItemWeight.RemoveItemFromPlace` _itemdata_placereferenceweight _itemdata))
    (:`Is Not Valid`
      (`/Engine/EditorBlueprintResources/StandardMacros.IsValid` _itemdata_placereferenceid
        (:`Is Valid`
          (`/Game/Main/Blueprints/PlaceForItemSystem/BP_PlaceForItemId.RemoveItemFromPlace` _itemdata_placereferenceid _itemdata))
        (:`Is Not Valid`
          _))))
  (bind _returnvalue (`|SpawnActorFromClass` "/Game/Main/Blueprints/InventorySystem/BP_Key.BP_Key_C" (`KismetMathLibrary.MakeTransform` (0.0 0.0 -10000.0)) "Undefined" "MultiplyWithRoot" null _itemdata null))
  (`self.DestroyItem`)
  (return _returnvalue))

(fn `UserConstructionScript`)