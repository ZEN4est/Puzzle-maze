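; Inventory component for the first-person character that stores item data and drives the inventory widget.
; AddItemToInventory appends the item's data, prints debug messages and passes the list to the widget.
; UnequipButton removes the widget's selected item from the list, then updates the widget.
; Description and refresh functions forward to the widget, each reached by casting the owner to BP_FirstPersonCharacter.
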(fn `AddItemToInventory`
  (params (ItemReference :type "/Game/Main/Blueprints/Inspection/BP_BaseItemToInspect Object Reference"))
  (bind _itemdata (`/Game/Main/Blueprints/Inspection/BP_BaseItemToInspect.ItemData` ItemReference))
  (bind _itemdata_itemname (break `/Game/Main/Blueprints/InventorySystem/S_InInventoryItem` (`/Game/Main/Blueprints/Inspection/BP_BaseItemToInspect.ItemData` ItemReference)))
  (bind _ininventoryitems (`self.InInventoryItems`))
  (`KismetSystemLibrary.PrintString` (`KismetTextLibrary.Conv_TextToString` _itemdata_itemname))
  (`KismetArrayLibrary.Array_Add` _ininventoryitems _itemdata)
  (`KismetSystemLibrary.PrintString` (`KismetStringLibrary.Concat_StrStr` "Item added: " (`KismetTextLibrary.Conv_TextToString` (`.ItemName_2_952662274EF6D6AF3FE2B4A93DC5D3CE` (break `/Game/Main/Blueprints/InventorySystem/S_InInventoryItem` _itemdata)))))
  (bind _asbp_first_person_character (cast `/Game/FirstPerson/Blueprints/BP_FirstPersonCharacter` (`self.GetOwner`)))
  (`/Game/Main/Blueprints/InventorySystem/W_Inventory.AddItemToList` (`/Game/FirstPerson/Blueprints/BP_FirstPersonCharacter.InventoryWidget` _asbp_first_person_character) ItemReference _ininventoryitems))

(fn `Inventory Refresh`
  (params (`Inventory Items` :type "Array of /Game/Main/Blueprints/InventorySystem/S_InInventoryItem Structure"))
  (bind _asbp_first_person_character (cast `/Game/FirstPerson/Blueprints/BP_FirstPersonCharacter` (`self.GetOwner`)))
  (`/Game/Main/Blueprints/InventorySystem/W_Inventory.InventoryRefresh` (`/Game/FirstPerson/Blueprints/BP_FirstPersonCharacter.InventoryWidget` _asbp_first_person_character) `Inventory Items`))

(fn `RemoveItemDescription`
  (bind _asbp_first_person_character (cast `/Game/FirstPerson/Blueprints/BP_FirstPersonCharacter` (`self.GetOwner`)))
  (`/Game/Main/Blueprints/InventorySystem/W_Inventory.ClearDescription` (`/Game/FirstPerson/Blueprints/BP_FirstPersonCharacter.InventoryWidget` _asbp_first_person_character)))

(fn `Show Item Descritpion`
  (params (SelectedItemReference :type "/Game/Main/Blueprints/InventorySystem/W_ItemSlot Object Reference"))
  (bind _asbp_first_person_character (cast `/Game/FirstPerson/Blueprints/BP_FirstPersonCharacter` (`self.GetOwner`)))
  (`/Game/Main/Blueprints/InventorySystem/W_Inventory.ShowItemDescription` (`/Game/FirstPerson/Blueprints/BP_FirstPersonCharacter.InventoryWidget` _asbp_first_person_character) SelectedItemReference))

(fn `UnequipButton`
  (bind _ininventoryitems (`self.InInventoryItems`))
  (bind _asbp_first_person_character (cast `/Game/FirstPerson/Blueprints/BP_FirstPersonCharacter` (`self.GetOwner`)))
  (bind _inventorywidget (`/Game/FirstPerson/Blueprints/BP_FirstPersonCharacter.InventoryWidget` _asbp_first_person_character))
  (`KismetArrayLibrary.Array_RemoveItem` _ininventoryitems (`/Game/Main/Blueprints/InventorySystem/W_ItemSlot.ItemData` (`/Game/Main/Blueprints/InventorySystem/W_Inventory.Selected Item Reference` _inventorywidget)))
  (`/Game/Main/Blueprints/InventorySystem/W_Inventory.UnequipItem` _inventorywidget _ininventoryitems))