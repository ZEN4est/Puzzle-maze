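; BP_InspectableObject is an actor for an inspectable object that shows an interaction prompt when looked at.
; Every tick it moves InteractIcon to a fixed height above the static mesh in world space and sets Interact's visibility from the LookedAt flag.
; The file never sets LookedAt, IsLookingAt always returns false, and the construction script only calls its parent.
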(event `self.ReceiveTick`
  (params (DeltaSeconds :type "Float (single-precision)"))
  (`SceneComponent.K2_SetWorldLocation` (`self.InteractIcon`) (+ (`SceneComponent.K2_GetComponentLocation` (`self.StaticMesh`)) (0.0 0.0 50.0)) false false)
  (if (`self.LookedAt?`)
    (`SceneComponent.SetVisibility` (`self.Interact`) true false)
    (else
      (`SceneComponent.SetVisibility` (`self.Interact`) false false))))

(fn `IsLookingAt?`
  (returns (`IsLookingAt?` :type Boolean))
  (return false))

(fn `UserConstructionScript`
  (`parent.UserConstructionScript`))