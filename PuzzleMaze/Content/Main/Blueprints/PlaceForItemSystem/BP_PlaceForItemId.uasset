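; Item placement spot that accepts the player's held item, if flagged as a random item, and checks whether its ID matches NeededId.
; Interacting while looking at its child BP_IconShowed removes the item from inventory and spawns it as a BP_Equipable on the pressure plate, briefly simulating physics.
; A match plays a confirmation sound; RemoveItemFromPlace clears the slot and rechecks.
; Tick sets the light green or red and toggles the icon.
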(event `self.ReceiveBeginPlay`
  (`self.EnableInput` (`GameplayStatics.GetPlayerController` 0))
  (bind _asbp_first_person_character (cast `/Game/FirstPerson/Blueprints/BP_FirstPersonCharacter` (`GameplayStatics.GetPlayerCharacter` 0)))
  (set `self.As BP First Person Character` _asbp_first_person_character)
  (bind _asbp_icon_showed (cast `/Game/Main/Blueprints/BP_IconShowed` (`self.IconShowedReference`)))
  (set `self.As BP Icon Showed` _asbp_icon_showed))

(event `RemoveItemFromPlace`
  (params (NewParam :type "/Game/Main/Blueprints/InventorySystem/S_InInventoryItem Structure (by ref)"))
  (bind (_object_itemname _object_itemdescription _object_itemicon _object_itemscale _object_itemrotation _object_itemmesh _object_icontransform _object_inspectionrotation _object_inspectionscale _object_keyid _object_itemid) (break `/Game/Main/Blueprints/InventorySystem/S_InInventoryItem` (`self.Object`)))
  (bind (_currentitemheld_itemname _currentitemheld_itemdescription _currentitemheld_itemicon _currentitemheld_itemscale _currentitemheld_itemrotation _currentitemheld_itemmesh _currentitemheld_icontransform _currentitemheld_inspectionrotation _currentitemheld_inspectionscale _currentitemheld_keyid _currentitemheld_itemid _currentitemheld_israndomitem_ _currentitemheld_placereferenceweight _currentitemheld_placereferenceid _currentitemheld_itemweight) (break `/Game/Main/Blueprints/InventorySystem/S_InInventoryItem` (`/Game/FirstPerson/Blueprints/BP_FirstPersonCharacter.CurrentItemHeld` (`self.As BP First Person Character`))))
  (set `/Game/FirstPerson/Blueprints/BP_FirstPersonCharacter.CurrentItemHeld` (make `/Game/Main/Blueprints/InventorySystem/S_InInventoryItem` _currentitemheld_itemname _currentitemheld_itemdescription _currentitemheld_itemicon _currentitemheld_itemscale (struct) _currentitemheld_itemmesh _currentitemheld_icontransform _currentitemheld_inspectionrotation _currentitemheld_inspectionscale _currentitemheld_keyid _currentitemheld_itemid _currentitemheld_israndomitem_ null null _currentitemheld_itemweight) (`self.As BP First Person Character`))
  (`KismetSystemLibrary.PrintString` "taken")
  (set `self.Object` (struct))
  (set `self.IsItemPlaced?` false)
  (if (== (`self.NeededId`) _object_itemid) :!label _label
    (set `self.ObjectConfirmed` true)
    (`GameplayStatics.SpawnSoundAtLocation` "/Game/Main/SFX/Confirmed.Confirmed" (`SceneComponent.K2_GetComponentLocation` (`self.DefaultSceneRoot`)) (struct) 2.0 1.0 0.0 "/Game/Main/Blueprints/NewSoundAttenuation.NewSoundAttenuation" null)
    (else
      (set `self.ObjectConfirmed` false))))

(event `EnhancedInput|/Game/FirstPerson/Input/Actions/IA_Interact`
  (params (ActionValue :type Boolean) (ElapsedSeconds :type "Float (double-precision)") (TriggeredSeconds :type "Float (double-precision)") (InputAction :type "InputAction Object Reference" :default "/Game/FirstPerson/Input/Actions/IA_Interact.IA_Interact"))
  (bind _as_bp_first_person_character (`self.As BP First Person Character`))
  (bind _as_bp_first_person_character_2 (`self.As BP First Person Character`))
  (bind (_currentitemheld_itemname _currentitemheld_itemdescription _currentitemheld_itemicon _currentitemheld_itemscale _currentitemheld_itemrotation _currentitemheld_itemmesh _currentitemheld_icontransform _currentitemheld_inspectionrotation _currentitemheld_inspectionscale _currentitemheld_keyid _currentitemheld_itemid _currentitemheld_israndomitem_) (break `/Game/Main/Blueprints/InventorySystem/S_InInventoryItem` (`/Game/FirstPerson/Blueprints/BP_FirstPersonCharacter.CurrentItemHeld` (`self.As BP First Person Character`))))
  (bind _currentitemheld (`/Game/FirstPerson/Blueprints/BP_FirstPersonCharacter.CurrentItemHeld` (`self.As BP First Person Character`)))
  (bind (_currentitemheld_itemname_2 _currentitemheld_itemdescription_2 _currentitemheld_itemicon_2 _currentitemheld_itemscale_2 _currentitemheld_itemrotation_2 _currentitemheld_itemmesh_2 _currentitemheld_icontransform_2 _currentitemheld_inspectionrotation_2 _currentitemheld_inspectionscale_2 _currentitemheld_keyid_2 _currentitemheld_itemid_2 _currentitemheld_israndomitem__2 _currentitemheld_placereferenceweight _currentitemheld_placereferenceid _currentitemheld_itemweight) (break `/Game/Main/Blueprints/InventorySystem/S_InInventoryItem` (`/Game/FirstPerson/Blueprints/BP_FirstPersonCharacter.CurrentItemHeld` (`self.As BP First Person Character`))))
  (:`Started`
    (if (`/Game/FirstPerson/Blueprints/BP_FirstPersonCharacter.IsHoldingItem?` (`self.As BP First Person Character`))
      (if (`/Game/Main/Blueprints/BP_IconShowed.LookingAt?` (`self.As BP Icon Showed`))
        (if (`self.IsItemPlaced?`)
          _
          (elif _currentitemheld_israndomitem_
            (`KismetArrayLibrary.Array_RemoveItem` (`/Game/Main/Blueprints/InventorySystem/BPC_Inventory.InInventoryItems` (`/Game/FirstPerson/Blueprints/BP_FirstPersonCharacter.BPC_Inventory` _as_bp_first_person_character)) (`/Game/FirstPerson/Blueprints/BP_FirstPersonCharacter.CurrentItemHeld` _as_bp_first_person_character))
            (set `/Game/FirstPerson/Blueprints/BP_FirstPersonCharacter.CurrentItemHeld` (make `/Game/Main/Blueprints/InventorySystem/S_InInventoryItem` _currentitemheld_itemname_2 _currentitemheld_itemdescription_2 _currentitemheld_itemicon_2 _currentitemheld_itemscale_2 (struct) _currentitemheld_itemmesh_2 _currentitemheld_icontransform_2 _currentitemheld_inspectionrotation_2 _currentitemheld_inspectionscale_2 _currentitemheld_keyid_2 _currentitemheld_itemid_2 _currentitemheld_israndomitem__2 null self _currentitemheld_itemweight) (`self.As BP First Person Character`))
            (bind _returnvalue (`|SpawnActorFromClass` "/Game/Main/Blueprints/InventorySystem/BP_Equipable.BP_Equipable_C" (`KismetMathLibrary.MakeTransform` (+ (`SceneComponent.GetSocketLocation` (`self.PressurePlate`) "None") (0.0 0.0 5.0))) "AlwaysSpawn" "MultiplyWithRoot" null _currentitemheld null))
            (`KismetSystemLibrary.PrintString` "Spawned")
            (set `self.Object` _currentitemheld)
            (set `self.IsItemPlaced?` true)
            (`StaticMeshComponent.SetStaticMesh` (`/Game/FirstPerson/Blueprints/BP_FirstPersonCharacter.InHandsItem` _as_bp_first_person_character_2) null)
            (set `/Game/FirstPerson/Blueprints/BP_FirstPersonCharacter.IsHoldingItem?` false _as_bp_first_person_character_2)
            (set `/Game/FirstPerson/Blueprints/BP_FirstPersonCharacter.CurrentItemHeld` (struct) _as_bp_first_person_character_2)
            (`/Game/Main/Blueprints/InventorySystem/BPC_Inventory.Inventory Refresh` (`/Game/FirstPerson/Blueprints/BP_FirstPersonCharacter.BPC_Inventory` (`self.As BP First Person Character`)) (`/Game/Main/Blueprints/InventorySystem/BPC_Inventory.InInventoryItems` (`/Game/FirstPerson/Blueprints/BP_FirstPersonCharacter.BPC_Inventory` (`self.As BP First Person Character`))))
            (bind _item (`/Game/Main/Blueprints/Inspection/BP_BaseItemToInspect.Item` _returnvalue))
            (`PrimitiveComponent.SetSimulatePhysics` _item true)
            (`KismetSystemLibrary.Delay` 0.2)
            (`PrimitiveComponent.SetSimulatePhysics` _item false)
            (goto _label)))))))

(event `self.ReceiveTick`
  (params (DeltaSeconds :type "Float (single-precision)"))
  (bind _lightindicator (`self.LightIndicator`))
  (bind (_currentitemheld_itemname _currentitemheld_itemdescription _currentitemheld_itemicon _currentitemheld_itemscale _currentitemheld_itemrotation _currentitemheld_itemmesh _currentitemheld_icontransform _currentitemheld_inspectionrotation _currentitemheld_inspectionscale _currentitemheld_keyid _currentitemheld_itemid _currentitemheld_israndomitem_) (break `/Game/Main/Blueprints/InventorySystem/S_InInventoryItem` (`/Game/FirstPerson/Blueprints/BP_FirstPersonCharacter.CurrentItemHeld` (`self.As BP First Person Character`))))
  (bind _returnvalue (`WidgetComponent.GetWidget` (`/Game/Main/Blueprints/BP_IconShowed.Widget` (`self.As BP Icon Showed`))))
  (if (`self.ObjectConfirmed`)
    (`LightComponent.SetLightColor` _lightindicator (make `LinearColor` 0.0 1.0 0.0 1.0) true)
    (else
      (`LightComponent.SetLightColor` _lightindicator (make `LinearColor` 1.0 0.0 0.0 1.0) true)))
  (if (`self.IsItemPlaced?`)
    (`Widget.SetVisibility` _returnvalue "Hidden" :!label _label_2)
    (elif (`/Game/FirstPerson/Blueprints/BP_FirstPersonCharacter.IsHoldingItem?` (`self.As BP First Person Character`))
      (if _currentitemheld_israndomitem_
        (`Widget.SetVisibility` _returnvalue "Visible"))
      (else
        (goto _label_2)))))

(fn `IsLookingAt?`
  (returns (`IsLookingAt?` :type Boolean))
  (return false))

(fn `UserConstructionScript`
  (bind _asbp_icon_showed (cast `/Game/Main/Blueprints/BP_IconShowed` (`ChildActorComponent.ChildActor` (`self.BP_IconShowed`))))
  (set `self.IconShowedReference` _asbp_icon_showed))