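; BP_ConnectPlaces links weight item places to a box and opens it when enough of them are confirmed.
; On BeginPlay it gathers BP_PlaceForItemWeight actors sharing its BoxReference, but sets the expected count from the loop index over all such actors, not the filtered array.
; Until confirmed, Tick recounts confirmed places each frame and calls OpenBox on the box when the count reaches that expected value.
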(event `self.ReceiveBeginPlay`
  (bind _outactors (`GameplayStatics.GetAllActorsOfClass` "/Game/Main/Blueprints/PlaceForItemSystem/BP_PlaceForItemWeight.BP_PlaceForItemWeight_C"))
  (for (_array_element _array_index) _outactors
    (if (== (`/Game/Main/Blueprints/PlaceForItemSystem/BP_PlaceForItemWeight.BoxReference` _array_element) (`self.BoxReference`))
      (`KismetArrayLibrary.Array_Add` (`self.PlacesArray`) _array_element)))
  (bind _output_get (set `self.ExpectedConfirmed` _array_index))
  (`KismetSystemLibrary.PrintString` (`KismetStringLibrary.Conv_IntToString` _output_get)))

(event `self.ReceiveTick`
  (params (DeltaSeconds :type "Float (single-precision)"))
  (if (not (`self.Confirmed`))
    (set `self.CurrentConfirmed` 0)
    (for _array_element (`self.PlacesArray`)
      (if (`/Game/Main/Blueprints/PlaceForItemSystem/BP_PlaceForItemWeight.ObjectConfirmed` _array_element)
        (set `self.CurrentConfirmed` (+ 1 (`self.CurrentConfirmed`)))
        (if (== (`self.CurrentConfirmed`) (`self.ExpectedConfirmed`))
          (set `self.Confirmed` true)
          (`KismetSystemLibrary.PrintString` "Box opened")
          (`/Game/Main/Blueprints/BP_Objects/BP_Box.OpenBox` (`self.BoxReference`))
          (else
            (set `self.Confirmed` false)))))
    (if true
      _)))

(fn `UserConstructionScript`)