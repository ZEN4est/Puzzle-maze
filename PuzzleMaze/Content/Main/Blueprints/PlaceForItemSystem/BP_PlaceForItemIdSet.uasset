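; BP_PlaceForItemIdSet is a puzzle actor that unlocks a door when three item slots all hold their correct objects.
; The construction script assigns a distinct required item ID to each of three child BP_PlaceForItemId actors.
; BeginPlay finds the BP_Door with a hard-coded key ID.
; Tick polls all three slots, unlocking that door when every one is confirmed and re-locking it otherwise.
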(event `self.ReceiveTick`
  (params (DeltaSeconds :type "Float (single-precision)"))
  (bind _doorreference (`self.DoorReference`))
  (bind _asbp_place_for_item_id (cast `/Game/Main/Blueprints/PlaceForItemSystem/BP_PlaceForItemId` (`ChildActorComponent.ChildActor` (`self.BP_PlaceForItemId`))))
  (bind _asbp_place_for_item_id_2 (cast `/Game/Main/Blueprints/PlaceForItemSystem/BP_PlaceForItemId` (`ChildActorComponent.ChildActor` (`self.BP_PlaceForItemId1`))))
  (bind _asbp_place_for_item_id_3 (cast `/Game/Main/Blueprints/PlaceForItemSystem/BP_PlaceForItemId` (`ChildActorComponent.ChildActor` (`self.BP_PlaceForItemId2`))))
  (if (`/Game/Main/Blueprints/PlaceForItemSystem/BP_PlaceForItemId.ObjectConfirmed` _asbp_place_for_item_id)
    (if (`/Game/Main/Blueprints/PlaceForItemSystem/BP_PlaceForItemId.ObjectConfirmed` _asbp_place_for_item_id_2)
      (if (`/Game/Main/Blueprints/PlaceForItemSystem/BP_PlaceForItemId.ObjectConfirmed` _asbp_place_for_item_id_3)
        (if (`/Game/Main/Blueprints/BP_Lockable.IsLocked` _doorreference)
          (`/Game/Main/Blueprints/BP_Objects/BP_Door.UnlockDorr` _doorreference))
        (else
          (set `/Game/Main/Blueprints/BP_Lockable.IsLocked` true _doorreference :!label _label)))
      (else
        (goto _label)))
    (else
      (goto _label))))

(event `self.ReceiveBeginPlay`
  (bind _outactors (`GameplayStatics.GetAllActorsOfClass` "/Game/Main/Blueprints/BP_Objects/BP_Door.BP_Door_C"))
  (for _array_element _outactors
    (if (== (`/Game/Main/Blueprints/BP_Objects/BP_Door.KeyId` _array_element) 10)
      (set `self.DoorReference` _array_element))))

(fn `UserConstructionScript`
  (bind _asbp_place_for_item_id (cast `/Game/Main/Blueprints/PlaceForItemSystem/BP_PlaceForItemId` (`ChildActorComponent.ChildActor` (`self.BP_PlaceForItemId`))))
  (set `/Game/Main/Blueprints/PlaceForItemSystem/BP_PlaceForItemId.NeededId` 11 _asbp_place_for_item_id)
  (bind _asbp_place_for_item_id_2 (cast `/Game/Main/Blueprints/PlaceForItemSystem/BP_PlaceForItemId` (`ChildActorComponent.ChildActor` (`self.BP_PlaceForItemId1`))))
  (set `/Game/Main/Blueprints/PlaceForItemSystem/BP_PlaceForItemId.NeededId` 13 _asbp_place_for_item_id_2)
  (bind _asbp_place_for_item_id_3 (cast `/Game/Main/Blueprints/PlaceForItemSystem/BP_PlaceForItemId` (`ChildActorComponent.ChildActor` (`self.BP_PlaceForItemId2`))))
  (set `/Game/Main/Blueprints/PlaceForItemSystem/BP_PlaceForItemId.NeededId` 12 _asbp_place_for_item_id_3))