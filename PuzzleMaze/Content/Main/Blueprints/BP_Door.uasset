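; Interactable door actor that the player opens and closes, and unlocks with a held key item whose KeyId matches.
; Look-at events store the player, and Tick checks the held item to show the Use, Open or Close prompt.
; IA_Interact with the matching key unlocks the door, removes the key from inventory and hands, and refreshes the inventory.
; Otherwise it toggles the unlocked door's animation, with a short delay blocking repeat input.
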(event `/Game/Main/Blueprints/Interfaces/BPI_LookAt.LookingAtActor`
  (params (PlayerReferemce :type "Actor Object Reference"))
  ;[1 1 1] LookingAt
  (set `self.Player Reference` PlayerReferemce)
  (set `self.LookingAt?` true))

(event `/Game/Main/Blueprints/Interfaces/BPI_LookAt.NoLookingAtActor`
  ;[1 1 1] LookingAt
  (set `self.Player Reference` null)
  (set `self.LookingAt?` false))

(event `self.ReceiveBeginPlay`
  (`self.EnableInput` (`GameplayStatics.GetPlayerController` 0)))

(event `self.ReceiveTick`
  (params (DeltaSeconds :type "Float (single-precision)"))
  (bind _player_reference (`self.Player Reference`))
  ;[1 1 1] ShowingInteraction
  (if (`self.LookingAt?`)
    (`/Engine/EditorBlueprintResources/StandardMacros.IsValid` _player_reference
      (:`Is Valid`
        (bind _asbp_first_person_character (cast `/Game/FirstPerson/Blueprints/BP_FirstPersonCharacter` _player_reference))
        (bind _asbp_equipable (cast `/Game/Main/Blueprints/InventorySystem/BP_Equipable` (`/Game/FirstPerson/Blueprints/BP_FirstPersonCharacter.CurrentItemHeld` _asbp_first_person_character))
          (:`then`
            (bind (_itemdata_itemname _itemdata_itemdescription _itemdata_itemicon _itemdata_itemscale _itemdata_itemmesh _itemdata_icontransform _itemdata_itemimage _itemdata_inspectionrotation _itemdata_inspectionscale _itemdata_keyid) (break `/Game/Main/Blueprints/InventorySystem/S_InInventoryItem` (`/Game/Main/Blueprints/Inspection/BP_BaseItemToInspect.ItemData` _asbp_equipable)))
            (bind _output_get (set `self.IsProperKey?` (== _itemdata_keyid (`self.KeyId`)))))
          (:`CastFailed`
            (set `self.IsProperKey?` false)))
        (if _output_get
          (if (`self.IsLocked`)
            (`SceneComponent.SetVisibility` (`self.E_Close`) false false)
            (`SceneComponent.SetVisibility` (`self.E_Open`) false false)
            (`SceneComponent.SetVisibility` (`self.E_Use`) true false)
            (else
              (`SceneComponent.SetVisibility` (`self.E_Use`) false false)))
          (elif (`self.IsLocked`)
            (`SceneComponent.SetVisibility` (`self.E_Use`) false false :!label _label)
            (`SceneComponent.SetVisibility` (`self.E_Close`) false false)
            (`SceneComponent.SetVisibility` (`self.E_Open`) false false)
            (else
              (`SceneComponent.SetVisibility` (`self.E_Use`) false false)
              (if (`self.IsOpen`) :!label _label_2
                (`SceneComponent.SetVisibility` (`self.E_Close`) true false)
                (`SceneComponent.SetVisibility` (`self.E_Open`) false false)
                (else
                  (`SceneComponent.SetVisibility` (`self.E_Open`) true false)
                  (`SceneComponent.SetVisibility` (`self.E_Close`) false false)))))))
      (:`Is Not Valid`
        (goto _label_2)))
    (else
      (goto _label))))

(event `EnhancedInput|/Game/FirstPerson/Input/Actions/IA_Interact`
  (params (ActionValue :type Boolean) (ElapsedSeconds :type "Float (double-precision)") (TriggeredSeconds :type "Float (double-precision)") (InputAction :type "InputAction Object Reference" :default "/Game/FirstPerson/Input/Actions/IA_Interact.IA_Interact"))
  (bind _player_reference (`self.Player Reference`))
  (:`Started`
    (if (`self.IsProperKey?`)
      ;[1 1 1] DoorOpening
      (set `self.IsLocked` false)
      ;[1 1 1] Removing from array
      (bind _asbp_first_person_character (cast `/Game/FirstPerson/Blueprints/BP_FirstPersonCharacter` _player_reference))
      (`KismetSystemLibrary.PrintString` "Ekwipunek przed:" true true (struct :`G` 0.66 :`B` 1.0 :`A` 1.0) 5.0)
      (bind _bpc_inventory (`/Game/FirstPerson/Blueprints/BP_FirstPersonCharacter.BPC_Inventory` _asbp_first_person_character))
      (bind _ininventoryitems (`/Game/Main/Blueprints/InventorySystem/BPC_Inventory.InInventoryItems` _bpc_inventory))
      (for _array_element _ininventoryitems
        (`KismetSystemLibrary.PrintString` (`KismetTextLibrary.Conv_TextToString` (break `/Game/Main/Blueprints/InventorySystem/S_InInventoryItem` _array_element)) true true (struct :`G` 0.66 :`B` 1.0 :`A` 1.0) 5.0))
      (bind _asbp_first_person_character_2 (cast `/Game/FirstPerson/Blueprints/BP_FirstPersonCharacter` _player_reference))
      (bind _asbp_equipable (cast `/Game/Main/Blueprints/InventorySystem/BP_Equipable` (`/Game/FirstPerson/Blueprints/BP_FirstPersonCharacter.CurrentItemHeld` _asbp_first_person_character_2)))
      (`KismetArrayLibrary.Array_RemoveItem` _ininventoryitems (`/Game/Main/Blueprints/Inspection/BP_BaseItemToInspect.ItemData` _asbp_equipable))
      (`KismetSystemLibrary.PrintString` "Ekwipunek po:" true true (struct :`G` 0.66 :`B` 1.0 :`A` 1.0) 5.0)
      (for _array_element_2 _ininventoryitems
        (`KismetSystemLibrary.PrintString` (`KismetTextLibrary.Conv_TextToString` (break `/Game/Main/Blueprints/InventorySystem/S_InInventoryItem` _array_element_2)) true true (struct :`G` 0.66 :`B` 1.0 :`A` 1.0) 5.0))
      ;[1 1 1] ClearInHandsItemMesh
      (bind _asbp_first_person_character_3 (cast `/Game/FirstPerson/Blueprints/BP_FirstPersonCharacter` (`self.Player Reference`)))
      (`StaticMeshComponent.SetStaticMesh` (`/Game/FirstPerson/Blueprints/BP_FirstPersonCharacter.InHandsItem` _asbp_first_person_character_3) null)
      (set `/Game/FirstPerson/Blueprints/BP_FirstPersonCharacter.IsHoldingItem?` false _asbp_first_person_character_3)
      (set `/Game/FirstPerson/Blueprints/BP_FirstPersonCharacter.CurrentItemHeld` null _asbp_first_person_character_3)
      (`/Game/Main/Blueprints/InventorySystem/BPC_Inventory.Inventory Refresh` _bpc_inventory _ininventoryitems)
      (elif (`self.LookingAt?`)
        (if (`self.IsLocked`)
          _
          (elif (not (`self.AnimationPlayed`))
            (if (`self.IsOpen`)
              ;;[1 1 1] Close
              (`SceneComponent.SetVisibility` (`self.E_Open`) true false)
              (`SceneComponent.SetVisibility` (`self.E_Close`) false false)
              (set `self.IsOpen` false)
              (`SkeletalMeshComponent.PlayAnimation` (`self.Door_0`) "/Game/Main/Objects/Door/Door_Anim_Armature_DoorClose.Door_Anim_Armature_DoorClose" false)
              (else
                ;;[1 1 1] Open
                (`SceneComponent.SetVisibility` (`self.E_Close`) true false)
                (`SceneComponent.SetVisibility` (`self.E_Open`) false false)
                (set `self.IsOpen` true)
                (`SkeletalMeshComponent.PlayAnimation` (`self.Door_0`) "/Game/Main/Objects/Door/Door_Anim_Armature_DoorOpen.Door_Anim_Armature_DoorOpen" false)))
            (set `self.AnimationPlayed` true)
            (`KismetSystemLibrary.Delay` 1.0)
            (set `self.AnimationPlayed` false)))))))

(fn `IsLookingAt?`
  (returns (`IsLookingAt?` :type Boolean))
  (return false))

(fn `UserConstructionScript`)