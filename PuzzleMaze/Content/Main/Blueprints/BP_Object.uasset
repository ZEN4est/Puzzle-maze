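; BP_Object is an object Blueprint that shows a spinning interaction indicator while it is being looked at.
; Every Tick it rotates the Interact and Interact1 components at a steady, frame-rate-independent speed and sets their visibility from the LookedAt flag.
; LookedAt is only read here, and the construction script just calls its parent.
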(event `self.ReceiveTick`
  (params (DeltaSeconds :type "Float (single-precision)"))
  (bind _returnvalue (* (struct :`Yaw` 90.0) DeltaSeconds))
  (`SceneComponent.K2_AddLocalRotation` (`self.Interact`) _returnvalue false false)
  (`SceneComponent.K2_AddLocalRotation` (`self.Interact1`) _returnvalue false false)
  (if (`self.LookedAt?`)
    (`SceneComponent.SetVisibility` (`self.Interact`) true false)
    (`SceneComponent.SetVisibility` (`self.Interact1`) true false)
    (else
      (`SceneComponent.SetVisibility` (`self.Interact`) false false)
      (`SceneComponent.SetVisibility` (`self.Interact1`) false false))))

(fn `UserConstructionScript`
  (`parent.UserConstructionScript`))