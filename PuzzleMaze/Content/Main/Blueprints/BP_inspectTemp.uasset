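; BP_inspectTemp is a temporary actor that presents a single item for inspection.
; Its Inspect event stores the character, sets the Item mesh and adds a W_Inspect widget showing the item's name and description.
; Both Inspect and the Interact press switch player-controller input with paired disable and enable calls.
; Pressing Interact also removes the widget, if valid, and destroys the actor.
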(event `/Game/Main/Blueprints/Interfaces/BPI_InteractTMP.Inspect`
  (params (Character :type "/Game/FirstPerson/Blueprints/BP_FirstPersonProjectile Object Reference") (InspectedItem :type "StaticMesh Object Reference") (ItemName :type Text) (ItemDescription :type Text))
  (bind _returnvalue (`GameplayStatics.GetPlayerController` 0))
  (set `self.Character` Character)
  (`StaticMeshComponent.SetStaticMesh` (`self.Item`) InspectedItem)
  (bind _returnvalue_2 (`|CreateWidget` "/Game/Main/Blueprints/W_Inspect.W_Inspect_C" null ItemName ItemDescription))
  (bind _output_get (set `self.InspectWidgetReference` _returnvalue_2))
  (`UserWidget.AddToViewport` _output_get 0)
  (`self.DisableInput` _returnvalue)
  (`self.EnableInput` _returnvalue))

(event `InputAction|Interact`
  (params (Key :type "Key Structure"))
  (bind _returnvalue (`GameplayStatics.GetPlayerController` 0))
  (bind _inspectwidgetreference (`self.InspectWidgetReference`))
  (:`Pressed`
    (`self.DisableInput` _returnvalue)
    (`self.EnableInput` _returnvalue)
    (`/Engine/EditorBlueprintResources/StandardMacros.IsValid` _inspectwidgetreference
      (:`Is Valid`
        (`Widget.RemoveFromParent` _inspectwidgetreference)
        (set `self.InspectWidgetReference` null)
        (`self.K2_DestroyActor`)))))

(fn `UserConstructionScript`)